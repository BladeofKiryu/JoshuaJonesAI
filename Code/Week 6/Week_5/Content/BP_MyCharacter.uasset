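; BP_MyCharacter is a player character with axis-driven movement, jumping and coin counting.
; Movement follows the control rotation's forward and right vectors.
; On Hit it destroys the other actor without filtering, then increments and prints Coins on the Manager game instance and loads a Week_5_2 level instance.
; Any actor overlap destroys the character itself.
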(event EventBeginPlay)

(event Collision|EventActorBeginOverlap
  (params (OtherActor :type Actor%20Object%20Reference))
  (Actor|DestroyActor))

(event EventTick
  (params (DeltaSeconds :type Float%20%28single-precision%29)))

(event Collision|EventHit
  (params (MyComp :type Primitive%20Component%20Object%20Reference) (Other :type Actor%20Object%20Reference) (OtherComp :type Primitive%20Component%20Object%20Reference) (bSelfMoved :type Boolean) (HitLocation :type Vector :default "0, 0, 0") (HitNormal :type Vector :default "0, 0, 0") (NormalImpulse :type Vector :default "0, 0, 0") (Hit :type Hit%20Result%20Structure%20%28by%20ref%29))
  (Actor|DestroyActor Other)
  (bind _asmanager (Utilities|Casting|CastToManager (Game|GetGameInstance)))
  (bind _output_get (Variables|/Game/Manager.Manager_C|SetCoins _asmanager (+ (Variables|/Game/Manager.Manager_C|GetCoins _asmanager) 1)))
  (Development|PrintString (Utilities|String|ToString(Integer) _output_get))
  (Class|LevelStreamingDynamic|LoadLevelInstance "Week_5_2" "0, 0, 0" "0, 0, 0"))

(event Input|ActionEvents|InputActionJump
  (params (Key :type Key%20Structure :default "None"))
  (:Pressed
    (Character|Jump)))

(event Input|AxisEvents|InputAxisMoveForward
  (params (AxisValue :type Float%20%28single-precision%29))
  (Pawn|Input|AddMovementInput (Math|Vector|GetForwardVector (Pawn|GetControlRotation :!class /Script/Engine.Pawn)) AxisValue false))

(event Input|AxisEvents|InputAxisMoveRight
  (params (AxisValue :type Float%20%28single-precision%29))
  (Pawn|Input|AddMovementInput (Math|Vector|GetRightVector (Pawn|GetControlRotation :!class /Script/Engine.Pawn)) AxisValue false))

(fn ConstructionScript)
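; Pong-style ball actor that bounces between player and enemy paddles and off walls using ProjectileMovement.
; Paddle overlaps reverse Y velocity and wall overlaps reverse Z, sharing a one-second cooldown.
; Tick returns the ball to a fixed point when it passes either paddle's Y, keeping only Y velocity.
; Paddle-direction spin is inactive: HandleBounce switches on constant zero instead of its input, and AddSpin's velocity change is disconnected.
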(event EventBeginPlay)

(event Collision|EventActorBeginOverlap
  (params (OtherActor :type Actor%20Object%20Reference))
  (bind _asplayerpaddle (Utilities|Casting|CastToplayerpaddle OtherActor)
    (:then
      (CallFunction|HandleBounce (Variables|/Game/playerpaddle.playerpaddle_C|Getmovedirection _asplayerpaddle)))
    (:CastFailed
      (bind _asenemypaddle (Utilities|Casting|CastToenemypaddle OtherActor)
        (:then
          (CallFunction|HandleBounce (Variables|/Game/enemypaddle.enemypaddle_C|Getmovedirection _asenemypaddle)))
        (:CastFailed
          (Utilities|Casting|CastToBP_Wall OtherActor)
          (CallFunction|ReverseZ))))))

(event EventTick
  (params (DeltaSeconds :type Float%20%28single-precision%29))
  (bind _projectilemovement (Variables|Default|GetProjectileMovement))
  (Variables|Default|SetTimeSinceReversed (+ DeltaSeconds (Variables|Default|GetTimeSinceReversed)))
  (bind _out_of_bounds (CallFunction|InOutofBounds))
  (if _out_of_bounds
    (Transformation|SetActorLocation "3950.000000, 0, 0" false false)
    (Variables|/Script/Engine.MovementComponent|SetVelocity _projectilemovement (Math|Vector|MakeVector 0.0 (.Y (Math|Vector|BreakVector (Variables|/Script/Engine.MovementComponent|GetVelocity _projectilemovement))) 0.0))))

(fn ConstructionScript)

(fn InOutofBounds
  (bind _outactors (Actor|GetAllActorsOfClass "/Game/playerpaddle.playerpaddle_C"))
  (if (<= (.Y (Math|Vector|BreakVector (Transformation|GetActorLocation))) (.Y (Math|Vector|BreakVector (Transformation|GetActorLocation (Utilities|Array|Get(acopy) _outactors)))))
    _
    (else
      (bind _outactors_2 (Actor|GetAllActorsOfClass "/Game/enemypaddle.enemypaddle_C"))
      (if (>= (.Y (Math|Vector|BreakVector (Transformation|GetActorLocation))) (.Y (Math|Vector|BreakVector (Transformation|GetActorLocation (Utilities|Array|Get(acopy) _outactors_2)))))
        _
        (else
          (return false)))))
  (return true))

(fn HandleBounce
  (params (selection :type Integer))
  (bind _returnvalue (Math|Random|RandomFloatinRange -5e+01 5e+01))
  (switch int 0
    (:-1
      (CallFunction|AddSpin (+ _returnvalue -125.0)))
    (:0
      (CallFunction|AddSpin (Math|Random|RandomFloatinRange -15.0 15.0)))
    (:1
      (CallFunction|AddSpin (+ _returnvalue 125.0))))
  (CallFunction|ReverseY))

(fn AddSpin
  (params (Spin :type Float%20%28single-precision%29)))

(fn ReverseY
  (if (>= (Variables|Default|GetTimeSinceReversed) 1.0)
    (Variables|/Script/Engine.MovementComponent|SetVelocity (Variables|Default|GetProjectileMovement) (Math|Vector|MakeVector (.X (Math|Vector|BreakVector (Variables|/Script/Engine.MovementComponent|GetVelocity (Variables|Default|GetProjectileMovement)))) (* -1 (.Y (Math|Vector|BreakVector (Variables|/Script/Engine.MovementComponent|GetVelocity (Variables|Default|GetProjectileMovement))))) (.Z (Math|Vector|BreakVector (Variables|/Script/Engine.MovementComponent|GetVelocity (Variables|Default|GetProjectileMovement))))))
    (Variables|Default|SetTimeSinceReversed 0.0)))

(fn ReverseZ
  (if (>= (Variables|Default|GetTimeSinceReversed) 1.0)
    (Variables|/Script/Engine.MovementComponent|SetVelocity (Variables|Default|GetProjectileMovement) (Math|Vector|MakeVector (.X (Math|Vector|BreakVector (Variables|/Script/Engine.MovementComponent|GetVelocity (Variables|Default|GetProjectileMovement)))) (.Y (Math|Vector|BreakVector (Variables|/Script/Engine.MovementComponent|GetVelocity (Variables|Default|GetProjectileMovement)))) (* -1 (.Z (Math|Vector|BreakVector (Variables|/Script/Engine.MovementComponent|GetVelocity (Variables|Default|GetProjectileMovement)))))))
    (Variables|Default|SetTimeSinceReversed 0.0)))